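; BP_Task_01_Actor is an interactable actor that toggles between active and inactive materials when interacted with and adds an on-screen marker widget for its location.
; While its collision sphere is overlapped, a looping timer refreshes interact prompt visibility instead of checking every tick.
; The range check, which also gates Interact, line-traces on the Camera channel to the first overlapping pawn to require an unobstructed path.
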(event `self.ReceiveBeginPlay`
  (bind _returnvalue (`|CreateWidget` (`self.MarkerWidgetClass`) (`GameplayStatics.GetPlayerController` 0)))
  (bind _output_get (set `self.MarkerWidget` _returnvalue))
  (message `/Game/Task_01/Blueprints/BPI_Marker.SetMarkerOriginLocation` _output_get (`self.K2_GetActorLocation`))
  (`UserWidget.AddToViewport` _output_get 0))

(event `/Game/Task_01/Blueprints/BPI_Interactable.Interact`
  (if (`self.IsPawnInInteractRange`)
    (`self.ToggleActive`)))

(event `self.SphereCollision.OnComponentBeginOverlap`
  (params (OverlappedComponent :type "PrimitiveComponent Object Reference") (OtherActor :type "Actor Object Reference") (OtherComp :type "PrimitiveComponent Object Reference") (OtherBodyIndex :type Integer) (bFromSweep :type Boolean) (SweepResult :type "HitResult Structure (by ref)"))
  (bind _returnvalue (`KismetSystemLibrary.K2_SetTimerDelegate` (`|CreateDelegate` :!event `CheckCollisionWithPawn`) (`self.CollisionCheckInterval`) true))
  (set `self.CollisionTimerHandle` _returnvalue))

(event `self.SphereCollision.OnComponentEndOverlap`
  (params (OverlappedComponent :type "PrimitiveComponent Object Reference") (OtherActor :type "Actor Object Reference") (OtherComp :type "PrimitiveComponent Object Reference") (OtherBodyIndex :type Integer))
  (`KismetSystemLibrary.K2_ClearAndInvalidateTimerHandle` (`self.CollisionTimerHandle`))
  (`self.SetInteractable` false))

(event `CheckCollisionWithPawn`
  (`self.SetInteractable` (`self.IsPawnInInteractRange`)))

(fn `IsPawnInInteractRange`
  (returns (bInRange :type Boolean))
  (locals (Pawn :type "Actor Object Reference"))
  (for _array_element (`PrimitiveComponent.GetOverlappingActors` (`self.SphereCollision`) "/Script/Engine.Pawn")
    (set `local.Pawn` _array_element)
    (bind _outhit (`KismetSystemLibrary.LineTraceSingle` (`self.K2_GetActorLocation`) (`self.K2_GetActorLocation` (`local.Pawn`)) "TraceTypeQuery2"))
    (return (== (`.HitActor` (`GameplayStatics.BreakHitResult` _outhit)) (`local.Pawn`)))))

(fn `SetInteractable`
  (params (bInteractable :type Boolean))
  (`SceneComponent.SetVisibility` (`self.InteractWidget`) bInteractable false)
  (return))

(fn `ToggleActive`
  (set `self.bActive` (not (`self.bActive`)))
  (`PrimitiveComponent.SetMaterial` (`self.Sphere`) 0 (select `bool` (`self.bActive`) :`false` (`self.MaterialInactive`) :`true` (`self.MaterialActive`)))
  (return))

(fn `UserConstructionScript`)