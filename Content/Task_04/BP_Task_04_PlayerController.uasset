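; Player controller for Task 04 that connects the W_Replication UI to its possessed character.
; On BeginPlay it creates the widget for the local controller only and binds its change-values and create-component delegates.
; Changing values calls ChangeValues on the cached BP_Task_04_Character, directly with authority or through ServerChangeValues when remote.
; The CreateDynamicComponent event is an empty stub.
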(event `self.ReceiveBeginPlay`
  (if (`self.IsLocalPlayerController`)
    (bind _returnvalue (`|CreateWidget` "/Game/Task_04/W_Replication.W_Replication_C"))
    (add `/Game/Task_04/W_Replication.OnChangeServerValues` _returnvalue (`|CreateDelegate` :!event `ChangeServerValues`))
    (add `/Game/Task_04/W_Replication.OnCreateDynamicComponent` _returnvalue (`|CreateDelegate` :!event `CreateDynamicComponent`))
    (`UserWidget.AddToViewport` _returnvalue 0)))

(event `self.ReceivePossess`
  (params (PossessedPawn :type "Pawn Object Reference"))
  (bind _asbp_task_04_character (cast `/Game/Task_04/BP_Task_04_Character` PossessedPawn))
  (set `self.BPCharacter` _asbp_task_04_character))

(event `ChangeServerValues`
  (`/Engine/EditorBlueprintResources/ActorMacros.Switch Has Authority`
    (:`Authority`
      (`/Game/Task_04/BP_Task_04_Character.ChangeValues` (`self.BPCharacter`)))
    (:`Remote`
      (`self.ServerChangeValues`))))

(event `ServerChangeValues`
  (`/Game/Task_04/BP_Task_04_Character.ChangeValues` (`self.BPCharacter`)))

(event `CreateDynamicComponent`)

(fn `UserConstructionScript`)